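; Fish pawn that carries an energy-driven light on the end of a cable.
; Each tick it optionally drains energy, eases the light radius toward it, hides a static mesh when energy is low and raises max speed as energy falls.
; Only the mesh turns to follow velocity, so its forward vector drives the cable force, with the light snapped to a cable particle.
; Foliage overlaps only print debug text; DamageTaken is an empty stub.
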(event `self.ReceiveTick`
  (params (DeltaSeconds :type "Float (single-precision)"))
  (if (`self.bDrainEnergyOverTime`)
    (`self.DrainEnergy` 50.0))
  (`self.UpdateEnergyLight`)
  (`self.CalcMaxSpeed`)
  (`self.LerpRotation`)
  (`self.UpdateCableEnd`))

(event `self.CollisionComponent.OnComponentBeginOverlap`
  (params (OverlappedComponent :type "PrimitiveComponent Object Reference") (OtherActor :type "Actor Object Reference") (OtherComp :type "PrimitiveComponent Object Reference") (OtherBodyIndex :type Integer) (bFromSweep :type Boolean) (SweepResult :type "HitResult Structure (by ref)"))
  ;[1 0 0] TODO: Check class instead of casting, also slow down movement speed
  (cast `InstancedFoliageActor` OtherActor)
  (`KismetSystemLibrary.PrintString` "Foliage Overlap" true true (struct :`G` 0.66 :`B` 1.0 :`A` 1.0) 0.0))

(event `self.CollisionComponent.OnComponentEndOverlap`
  (params (OverlappedComponent :type "PrimitiveComponent Object Reference") (OtherActor :type "Actor Object Reference") (OtherComp :type "PrimitiveComponent Object Reference") (OtherBodyIndex :type Integer))
  ;[1 0 0] TODO: Check class instead of casting, also slow down movement speed
  (cast `InstancedFoliageActor` OtherActor)
  (`KismetSystemLibrary.PrintString` "Foliage EndOverlap" true true (struct :`G` 0.66 :`B` 1.0 :`A` 1.0) 0.0))

(fn `CalcMaxSpeed`
  (set `FloatingPawnMovement.MaxSpeed` (- (`self.MaxSpeed`) (* (/ (`self.CurrentEnergy`) (`self.MaxEnergy`)) (- (`self.MaxSpeed`) (`self.MinSpeed`)))) (`self.FloatingPawnMovement`)))

(fn `DamageTaken`
  (params (From :type "/Game/FishyJam/Core/Enemy/BP_FishyEnemy Object Reference") (Amount :type "Float (double-precision)")))

(fn `DrainEnergy`
  (params (Amount :type "Float (double-precision)"))
  (set `self.CurrentEnergy` (`KismetMathLibrary.FClamp` (- (`self.CurrentEnergy`) (* Amount (`GameplayStatics.GetWorldDeltaSeconds`))) 0.0 (`self.MaxEnergy`))))

(fn `LerpRotation`
  (bind _mesh (`self.Mesh`))
  (bind (_returnvalue_x _returnvalue_y) (`KismetMathLibrary.BreakVector` (`KismetMathLibrary.Conv_RotatorToVector` (`self.K2_GetActorRotation`))))
  (bind (_velocity_x _velocity_y) (`KismetMathLibrary.BreakVector` (`MovementComponent.Velocity` (`self.FloatingPawnMovement`))))
  (if (!= (`MovementComponent.Velocity` (`self.FloatingPawnMovement`)) (0.0 0.0 0.0))
    (if (== (`KismetMathLibrary.CrossProduct2D` (`KismetMathLibrary.MakeVector2D` _velocity_x _velocity_y) (`KismetMathLibrary.MakeVector2D` _returnvalue_x _returnvalue_y)) 0.0)
      (`|ExecutionSequence`
        (:`then_0`
          (`SceneComponent.K2_AddRelativeRotation` _mesh (struct :`Yaw` 0.01) false false) ; if we look straight up or down, add a little more delta rot
        )
        (:`then_1`
          _)))
    (`SceneComponent.K2_SetRelativeRotation` _mesh (`KismetMathLibrary.Conv_VectorToRotator` (`KismetMathLibrary.Normal` (`KismetMathLibrary.VLerp` (`KismetMathLibrary.Conv_RotatorToVector` (`SceneComponent.RelativeRotation` (`self.Mesh`))) (`KismetMathLibrary.Normal` (`|Copy` (`MovementComponent.Velocity` (`self.FloatingPawnMovement`)))) 0.2))) false false) ; Need to lerp instead
  ))

(fn `UpdateCableEnd`
  (bind _cable (`self.Cable`))
  (`SceneComponent.K2_SetWorldLocation` (`self.EnergyLight`) (`|GetArrayItem` (`CableComponent.GetCableParticleLocations` _cable) 10) false true)
  ;[1 1 1] Hack, because Actor Rotation is not moving at all, only the mesh
  (set `CableComponent.CableForce` (* (`SceneComponent.GetForwardVector` (`self.Mesh`)) 50000.0) _cable))

(fn `UpdateEnergyLight`
  (bind _currentenergy (`self.CurrentEnergy`))
  (bind _energylight (`self.EnergyLight`))
  (`PointLightComponent.SetAttenuationRadius` _energylight (`KismetMathLibrary.Lerp` (`PointLightComponent.AttenuationRadius` _energylight) _currentenergy 0.1))
  (`SceneComponent.SetHiddenInGame` (`self.StaticMesh`) (< _currentenergy 280.0) false))

(fn `UserConstructionScript`
  (`self.UpdateCableEnd`))