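; Game mode for Fishy Jam that runs enemy spawning, the anti-idle penalty and game over.
; A self-rescheduling one-second timer periodically adds off-screen Haunt and Patrol enemy pairs up to a cap; its enemy speed check is an empty stub.
; Tick spawns a piranha group off-screen when the player swims too slowly for three seconds.
; Tick also polls for BP_FishyFriend actors, disabling input and showing the game-over widget when none remain.
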(event `self.ReceiveBeginPlay`
  (`self.SpawnEnemies` 4) ; Initial Enemy Spawn
  (`self.TimePassedCounter`))

(event `self.ReceiveTick`
  (params (DeltaSeconds :type "Float (single-precision)"))
  (`self.HandleTooSlow`)
  (`self.CheckForGameOver`))

(event `DefaultTimer`
  (`self.CheckSpawnNewEnemy` 10)
  (`self.CheckModifyEnemySpeed` 10))

(fn `CheckForGameOver`
  (bind _outactors (`GameplayStatics.GetAllActorsOfClass` "/Game/FishyJam/Core/Interactables/BP_FishyFriend.BP_FishyFriend_C"))
  (if (== (`KismetArrayLibrary.Array_Length` _outactors) 0)
    (`self.HandleGameOver`)))

(fn `CheckModifyEnemySpeed`
  (params (`ModifyEveryX Seconds` :type Integer))
  (if (== (mod (`self.TimePassedSeconds`) `ModifyEveryX Seconds`) 0)
    _))

(fn `CheckSpawnNewEnemy`
  (params (`SpawnEveryX Seconds` :type Integer))
  (if (and (== (mod (`self.TimePassedSeconds`) `SpawnEveryX Seconds`) 0) (<= (+ (`KismetArrayLibrary.Array_Length` (`self.Enemies`)) 2) (`self.EnemyCap`)))
    (`self.SpawnEnemies` 1)))

(fn `GetRandomEnemySpawnLocation`
  (params (Boundary :type "Float (double-precision)"))
  (returns (Location :type "Vector Structure"))
  (locals (InBoundary :type "Float (double-precision)") (PlayerLocation :type "Vector Structure"))
  (bind (_playerlocation_x _playerlocation_y) (`KismetMathLibrary.BreakVector` (`local.PlayerLocation`)))
  (bind _playerlocation_x_2 (`KismetMathLibrary.BreakVector` (`local.PlayerLocation`)))
  (bind _returnvalue (/ (`.SizeY` (`PlayerController.GetViewportSize` (`GameplayStatics.GetPlayerController` 0))) 2))
  (bind _returnvalue_2 (/ (`PlayerController.GetViewportSize` (`GameplayStatics.GetPlayerController` 0)) 2))
  (set `local.InBoundary` Boundary)
  (set `local.PlayerLocation` (`self.K2_GetActorLocation` (`Controller.K2_GetPawn` (`GameplayStatics.GetPlayerController` 0))))
  (return (`KismetMathLibrary.MakeVector` (`KismetMathLibrary.SelectFloat` (`KismetMathLibrary.RandomFloatInRange` (* -1 (`KismetMathLibrary.Abs` (`local.InBoundary`))) (+ (`KismetMathLibrary.Conv_IntToDouble` (* _returnvalue_2 -1)) _playerlocation_x_2)) (`KismetMathLibrary.RandomFloatInRange` (+ _playerlocation_x_2 (`KismetMathLibrary.Conv_IntToDouble` _returnvalue_2)) (`KismetMathLibrary.Abs` (`local.InBoundary`))) (`KismetMathLibrary.RandomBool`)) (`KismetMathLibrary.SelectFloat` (`KismetMathLibrary.RandomFloatInRange` (* -1 (`KismetMathLibrary.Abs` (`local.InBoundary`))) (+ (`KismetMathLibrary.Conv_IntToDouble` (* _returnvalue -1)) _playerlocation_y)) (`KismetMathLibrary.RandomFloatInRange` (+ _playerlocation_y (`KismetMathLibrary.Conv_IntToDouble` _returnvalue)) (`KismetMathLibrary.Abs` (`local.InBoundary`))) (`KismetMathLibrary.RandomBool`)) 250.0)))

(fn `HandleGameOver`
  (bind _returnvalue (`GameplayStatics.GetPlayerController` 0))
  (if (not (`self.bGameOver`))
    (set `self.bGameOver` true)
    (`self.DisableInput` (`Controller.K2_GetPawn` _returnvalue) _returnvalue)
    (bind _returnvalue_2 (`|CreateWidget` "/Game/FishyJam/UI/WBP_GameOver.WBP_GameOver_C"))
    (`UserWidget.AddToViewport` _returnvalue_2 0)
    (`WidgetBlueprintLibrary.SetInputMode_GameAndUIEx` _returnvalue _returnvalue_2)
    (set `PlayerController.bShowMouseCursor` true _returnvalue)))

(fn `HandleTooSlow`
  (locals (OutOfViewportPos :type "Vector Structure") (FishyPawn :type "/Game/FishyJam/Core/Pawns/BP_FishyPawn Object Reference"))
  (bind (_returnvalue_x _returnvalue_y) (`KismetMathLibrary.BreakVector2D` (`WidgetLayoutLibrary.GetViewportSize`)))
  ;[1 1 1] Check if player swims too slow
  (bind _asbp_fishy_pawn (cast `/Game/FishyJam/Core/Pawns/BP_FishyPawn` (`Controller.K2_GetPawn` (`GameplayStatics.GetPlayerController` 0))))
  (set `local.FishyPawn` _asbp_fishy_pawn)
  (if (< (`KismetMathLibrary.VSize` (`self.GetVelocity` _asbp_fishy_pawn)) (`self.TooSlowThreshold`))
    ;[1 1 1] Check whether its time to spawn the piranhas
    (if (not (`self.bHasSpawnedPiranhas`))
      (if (>= (`self.TooSlowTime`) 3.0)
        ;[1 1 1] Find Spawn Position
        (set `local.OutOfViewportPos` (+ (`self.K2_GetActorLocation` (`local.FishyPawn`)) (`KismetMathLibrary.MakeVector` (* (`KismetMathLibrary.SelectFloat` -1.0 1.0 (`KismetMathLibrary.RandomBool`)) _returnvalue_x) (* _returnvalue_y (`KismetMathLibrary.SelectFloat` -1.0 1.0 (`KismetMathLibrary.RandomBool`))))))
        ;[1 1 1] Spawn
        (for _ (range (+ (`self.NumSpawnPiranha`) 1))
          (`|SpawnActorFromClass` "/Game/FishyJam/Core/Enemy/BP_FishyEnemyPiranha.BP_FishyEnemyPiranha_C" (`KismetMathLibrary.MakeTransform` (+ (`local.OutOfViewportPos`) (`KismetMathLibrary.MakeVector` (`KismetMathLibrary.RandomFloatInRange` 0.0 200.0) (`KismetMathLibrary.RandomFloatInRange` 0.0 200.0)))) "AlwaysSpawn" "OverrideRootScale" null null))
        (set `self.bHasSpawnedPiranhas` true)
        (else
          (set `self.TooSlowTime` (+ (`self.TooSlowTime`) (`GameplayStatics.GetWorldDeltaSeconds`))))))
    (else
      (set `self.TooSlowTime` 0.0)
      (set `self.bHasSpawnedPiranhas` false))))

(fn `SpawnEnemies`
  (params (Num :type Integer))
  (bind _enemies (`self.Enemies`))
  (if (> Num 0)
    (for _ (range (+ Num 1))
      (`|ExecutionSequence`
        (:`then_0`
          (bind _location (`self.GetRandomEnemySpawnLocation` 3000.0))
          (bind _returnvalue (`|SpawnActorFromClass` "/Game/FishyJam/Core/Enemy/BP_FishyEnemyHaunt.BP_FishyEnemyHaunt_C" (`KismetMathLibrary.MakeTransform` _location) "Undefined" "OverrideRootScale" null null))
          (`KismetArrayLibrary.Array_Add` _enemies _returnvalue))
        (:`then_1`
          (bind _location_2 (`self.GetRandomEnemySpawnLocation` 3000.0))
          (bind _returnvalue_2 (`|SpawnActorFromClass` "/Game/FishyJam/Core/Enemy/BP_FishyEnemyPatrol.BP_FishyEnemyPatrol_C" (`KismetMathLibrary.MakeTransform` _location_2) "Undefined" "OverrideRootScale" null null))
          (`KismetArrayLibrary.Array_Add` _enemies _returnvalue_2))))))

(fn `TimePassedCounter`
  (`/Engine/EditorBlueprintResources/StandardMacros.IncrementInt` (`self.TimePassedSeconds`)
    (:`  `
      (`self.DefaultTimer`)
      (`KismetSystemLibrary.K2_SetTimer` self "TimePassedCounter" 1.0))))

(fn `TooSlowSpawnLocation`
  (returns (SpawnLocation :type "Vector Structure"))
  (cast `/Game/FishyJam/Core/Pawns/BP_FishyPawn` (`Controller.K2_GetPawn` (`GameplayStatics.GetPlayerController` 0))
    (:`then`
      (`KismetSystemLibrary.PrintString` "Hello")
      (return (0.0 0.0 0.0)))
    (:`CastFailed`
      (return (0.0 0.0 0.0)))))

(fn `UserConstructionScript`)