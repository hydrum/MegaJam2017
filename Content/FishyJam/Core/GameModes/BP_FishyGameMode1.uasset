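; BP_FishyGameMode1 is a fish game's game mode that punishes slow swimming and detects game over.
; Each tick, it times low pawn velocity and, after three seconds, spawns one piranha group at a random diagonal offset scaled by viewport size, rearming when speed recovers.
; It also polls for BP_FishyFriend actors; when none remain, it disables pawn input and shows WBP_GameOver.
; TooSlowSpawnLocation is an unused stub.
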(event `self.ReceiveTick`
  (params (DeltaSeconds :type "Float (single-precision)"))
  (`self.HandleTooSlow`)
  (`self.CheckForGameOver`))

(fn `CheckForGameOver`
  (bind _outactors (`GameplayStatics.GetAllActorsOfClass` "/Game/FishyJam/Core/Interactables/BP_FishyFriend.BP_FishyFriend_C"))
  (if (== (`KismetArrayLibrary.Array_Length` _outactors) 0)
    (`self.HandleGameOver`)))

(fn `HandleGameOver`
  (bind _returnvalue (`GameplayStatics.GetPlayerController` 0))
  (if (not (`self.bGameOver`))
    (set `self.bGameOver` true)
    (`self.DisableInput` (`Controller.K2_GetPawn` _returnvalue) _returnvalue)
    (bind _returnvalue_2 (`|CreateWidget` "/Game/FishyJam/UI/WBP_GameOver.WBP_GameOver_C"))
    (`UserWidget.AddToViewport` _returnvalue_2 0)
    (`WidgetBlueprintLibrary.SetInputMode_UIOnlyEx` _returnvalue _returnvalue_2)
    (set `PlayerController.bShowMouseCursor` true _returnvalue)))

(fn `HandleTooSlow`
  (locals (OutOfViewportPos :type "Vector Structure") (FishyPawn :type "/Game/FishyJam/Core/Pawns/BP_FishyPawn Object Reference"))
  (bind (_returnvalue_x _returnvalue_y) (`KismetMathLibrary.BreakVector2D` (`WidgetLayoutLibrary.GetViewportSize`)))
  ;[1 1 1] Check if player swims too slow
  (bind _asbp_fishy_pawn (cast `/Game/FishyJam/Core/Pawns/BP_FishyPawn` (`Controller.K2_GetPawn` (`GameplayStatics.GetPlayerController` 0))))
  (set `local.FishyPawn` _asbp_fishy_pawn)
  (if (< (`KismetMathLibrary.VSize` (`self.GetVelocity` _asbp_fishy_pawn)) (`self.TooSlowThreshold`))
    ;[1 1 1] Check whether its time to spawn the piranhas
    (if (not (`self.bHasSpawnedPiranhas`))
      (if (>= (`self.TooSlowTime`) 3.0)
        ;[1 1 1] Find Spawn Position
        (set `local.OutOfViewportPos` (+ (`self.K2_GetActorLocation` (`local.FishyPawn`)) (`KismetMathLibrary.MakeVector` (* (`KismetMathLibrary.SelectFloat` -1.0 1.0 (`KismetMathLibrary.RandomBool`)) _returnvalue_x) (* _returnvalue_y (`KismetMathLibrary.SelectFloat` -1.0 1.0 (`KismetMathLibrary.RandomBool`))))))
        ;[1 1 1] Spawn
        (for _ (range (+ (`self.NumSpawnPiranha`) 1))
          (`|SpawnActorFromClass` "/Game/FishyJam/Core/Enemy/BP_FishyEnemyPiranha.BP_FishyEnemyPiranha_C" (`KismetMathLibrary.MakeTransform` (+ (`local.OutOfViewportPos`) (`KismetMathLibrary.MakeVector` (`KismetMathLibrary.RandomFloatInRange` 0.0 200.0) (`KismetMathLibrary.RandomFloatInRange` 0.0 200.0)))) "AlwaysSpawn" "OverrideRootScale" null null))
        (set `self.bHasSpawnedPiranhas` true)
        (else
          (set `self.TooSlowTime` (+ (`self.TooSlowTime`) (`GameplayStatics.GetWorldDeltaSeconds`))))))
    (else
      (set `self.TooSlowTime` 0.0)
      (set `self.bHasSpawnedPiranhas` false))))

(fn `TooSlowSpawnLocation`
  (returns (SpawnLocation :type "Vector Structure"))
  (cast `/Game/FishyJam/Core/Pawns/BP_FishyPawn` (`Controller.K2_GetPawn` (`GameplayStatics.GetPlayerController` 0))
    (:`then`
      (`KismetSystemLibrary.PrintString` "Hello")
      (return (0.0 0.0 0.0)))
    (:`CastFailed`
      (return (0.0 0.0 0.0)))))

(fn `UserConstructionScript`)