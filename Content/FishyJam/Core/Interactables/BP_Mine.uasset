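; BP_Mine is an interactable hazard that damages the player fish on contact in FishyJam.
; When a BP_FishyPawn overlaps its Sphere1 trigger, it subtracts half the pawn's maximum energy from its current energy.
; It then attaches an explosion particle to its Sphere component and destroys itself after a short delay.
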(event `self.Sphere1.OnComponentBeginOverlap`
  (params (OverlappedComponent :type "PrimitiveComponent Object Reference") (OtherActor :type "Actor Object Reference") (OtherComp :type "PrimitiveComponent Object Reference") (OtherBodyIndex :type Integer) (bFromSweep :type Boolean) (SweepResult :type "HitResult Structure (by ref)"))
  (bind _asbp_fishy_pawn (cast `/Game/FishyJam/Core/Pawns/BP_FishyPawn` OtherActor))
  (set `/Game/FishyJam/Core/BP_FishyFish.CurrentEnergy` (- (`/Game/FishyJam/Core/BP_FishyFish.CurrentEnergy` _asbp_fishy_pawn) (/ (`/Game/FishyJam/Core/BP_FishyFish.MaxEnergy` _asbp_fishy_pawn) 2.0)) _asbp_fishy_pawn)
  (`GameplayStatics.SpawnEmitterAttached` (`self.Explosion Particle`) (`self.Sphere`))
  (`KismetSystemLibrary.Delay` 0.2)
  (`self.K2_DestroyActor`))

(fn `UserConstructionScript`)