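; BP_RockWall is an interactable rock wall that sinks 600 units from its starting position once it is unlocked and the tutorial is enabled.
; From BeginPlay it polls every 0.2 seconds, reading TutorialEnabled from the first BP_MenuLevel actor alongside its own IsUnlocked flag.
; When both are true, polling stops and a timeline lerps the wall down without sweeping.
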(event `LoopTutorialCheck`
  (bind _outactors (`GameplayStatics.GetAllActorsOfClass` "/Game/FishyJam/Core/Interactables/BP_MenuLevel.BP_MenuLevel_C" :!label _label))
  (bind _output_get (set `self.MenuLevelReference` (`|GetArrayItem` _outactors)))
  (if (and (`/Game/FishyJam/Core/Interactables/BP_MenuLevel.TutorialEnabled` _output_get) (`self.IsUnlocked`))
    (bind (_direction _newtrack_0) (`Timeline|Timeline_0` :!via `PlayFromStart`)
      (:`Update`
        (`self.K2_SetActorLocation` (`KismetMathLibrary.VLerp` (`self.StartLocation`) (`self.EndLocation`) _newtrack_0))))
    (else
      (`KismetSystemLibrary.Delay` 0.2)
      (`self.LoopTutorialCheck`))))

(event `self.ReceiveBeginPlay`
  (bind _output_get (set `self.StartLocation` (`self.K2_GetActorLocation` self)))
  (set `self.EndLocation` (- _output_get (0.0 0.0 600.0)))
  (goto _label))

(fn `UserConstructionScript`)