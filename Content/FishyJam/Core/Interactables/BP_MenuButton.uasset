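; World-space menu button that the player's fish pawn activates by staying inside its activation radius until its energy is full.
; Overlap starts a delayed polling loop that dispatches on ButtonFunction to open a level, quit, or enable the tutorial on BP_MenuLevel.
; The loop keeps running after exit, with each action gated by the overlap flag and full energy.
; The construction script sets the label text; Options is an empty stub.
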(event `LoopFunctionActivation`
  (switch `/Game/FishyJam/Core/Interactables/Enum_MenuFuctions` (`self.ButtonFunction`) :!label _label
    (:`NewEnumerator0`
      (`self.LoadLevel`))
    (:`NewEnumerator1`
      (`self.OpenSettings`))
    (:`NewEnumerator2`
      (`self.QuitGame`))
    (:`NewEnumerator3`
      (`self.PlayTutorial`)))
  (`KismetSystemLibrary.Delay` 0.2)
  (`self.LoopFunctionActivation`))

(event `self.ActivationRadius.OnComponentBeginOverlap`
  (params (OverlappedComponent :type "PrimitiveComponent Object Reference") (OtherActor :type "Actor Object Reference") (OtherComp :type "PrimitiveComponent Object Reference") (OtherBodyIndex :type Integer) (bFromSweep :type Boolean) (SweepResult :type "HitResult Structure (by ref)"))
  (if (== OtherActor (`GameplayStatics.GetPlayerPawn` 0))
    (set `self.PawnReference` null)
    (set `self.IsOverlapping` true)
    (goto _label)))

(event `self.ActivationRadius.OnComponentEndOverlap`
  (params (OverlappedComponent :type "PrimitiveComponent Object Reference") (OtherActor :type "Actor Object Reference") (OtherComp :type "PrimitiveComponent Object Reference") (OtherBodyIndex :type Integer))
  (if (== OtherActor (`GameplayStatics.GetPlayerPawn` 0))
    (set `self.IsOverlapping` false)))

(fn `LoadLevel`
  (if (`self.IsOverlapping`)
    (bind _outactors (`GameplayStatics.GetAllActorsOfClass` "/Game/FishyJam/Core/Pawns/BP_FishyPawn.BP_FishyPawn_C"))
    (bind _output (`|GetArrayItem` _outactors))
    (if (== (`/Game/FishyJam/Core/BP_FishyFish.CurrentEnergy` _output) (`/Game/FishyJam/Core/BP_FishyFish.MaxEnergy` _output))
      (`GameplayStatics.OpenLevel` (`self.LevelName`)))))

(fn `OpenSettings`)

(fn `PlayTutorial`
  (if (`self.IsOverlapping`)
    (bind _outactors (`GameplayStatics.GetAllActorsOfClass` "/Game/FishyJam/Core/Pawns/BP_FishyPawn.BP_FishyPawn_C"))
    (bind _output (`|GetArrayItem` _outactors))
    (if (== (`/Game/FishyJam/Core/BP_FishyFish.CurrentEnergy` _output) (`/Game/FishyJam/Core/BP_FishyFish.MaxEnergy` _output))
      (bind _outactors_2 (`GameplayStatics.GetAllActorsOfClass` "/Game/FishyJam/Core/Interactables/BP_MenuLevel.BP_MenuLevel_C"))
      (bind _output_get (set `self.MenuLevelReference` (`|GetArrayItem` _outactors_2)))
      (set `/Game/FishyJam/Core/Interactables/BP_MenuLevel.TutorialEnabled` true _output_get))))

(fn `QuitGame`
  (if (`self.IsOverlapping`)
    (bind _outactors (`GameplayStatics.GetAllActorsOfClass` "/Game/FishyJam/Core/Pawns/BP_FishyPawn.BP_FishyPawn_C"))
    (bind _output (`|GetArrayItem` _outactors))
    (if (== (`/Game/FishyJam/Core/BP_FishyFish.CurrentEnergy` _output) (`/Game/FishyJam/Core/BP_FishyFish.MaxEnergy` _output))
      (`KismetSystemLibrary.QuitGame` (`GameplayStatics.GetPlayerController` 0) "Quit"))))

(fn `UserConstructionScript`
  (`TextRenderComponent.K2_SetText` (`self.TextRender`) (`self.Text`)))