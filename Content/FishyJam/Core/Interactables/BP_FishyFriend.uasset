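; BP_FishyFriend is an interactable friend fish that takes energy from the player's BP_FishyPawn while it is nearby.
; Overlapping InteractableZone stores the pawn and flags charging, and leaving the zone clears both.
; While charging, Tick calls DrainEnergy with opposite signs on itself and the pawn, moving a fixed amount per call without Delta Seconds scaling in this Blueprint.
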(event `self.ReceiveTick`
  (params (DeltaSeconds :type "Float (single-precision)"))
  (`parent.ReceiveTick` DeltaSeconds)
  (`self.ChargeFishyFriend`))

(event `self.InteractableZone.OnComponentBeginOverlap`
  (params (OverlappedComponent :type "PrimitiveComponent Object Reference") (OtherActor :type "Actor Object Reference") (OtherComp :type "PrimitiveComponent Object Reference") (OtherBodyIndex :type Integer) (bFromSweep :type Boolean) (SweepResult :type "HitResult Structure (by ref)"))
  (bind _asbp_fishy_pawn (cast `/Game/FishyJam/Core/Pawns/BP_FishyPawn` OtherActor))
  (set `self.FishyPawn` _asbp_fishy_pawn)
  (set `self.bIsChargingFriend` true))

(event `self.InteractableZone.OnComponentEndOverlap`
  (params (OverlappedComponent :type "PrimitiveComponent Object Reference") (OtherActor :type "Actor Object Reference") (OtherComp :type "PrimitiveComponent Object Reference") (OtherBodyIndex :type Integer))
  (cast `/Game/FishyJam/Core/Pawns/BP_FishyPawn` OtherActor)
  (set `self.FishyPawn` null)
  (set `self.bIsChargingFriend` false))

(fn `ChargeFishyFriend`
  (if (`self.bIsChargingFriend`)
    (`/Engine/EditorBlueprintResources/StandardMacros.IsValid` (`self.FishyPawn`)
      (:`Is Valid`
        (`self.DrainEnergy` -200.0)
        (`self.DrainEnergy` (`self.FishyPawn`) 200.0)))))

(fn `UserConstructionScript`
  (`parent.UserConstructionScript`))