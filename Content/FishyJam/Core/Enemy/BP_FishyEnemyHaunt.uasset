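; Haunting enemy fish, a child enemy Blueprint that pursues the HauntedFish and is repelled by its light.
; Tick prioritizes charging, then panicking, then swimming away during attack cooldown, otherwise swimming toward the target.
; Entering light range starts a panic away from it over a random distance, cleared on wall hit.
; Outside the light, CheckFishInRange starts a charge at the haunted fish when close, otherwise at a nearby FishyFriend.
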(event `self.ReceiveTick`
  (params (DeltaSeconds :type "Float (single-precision)"))
  ;[1 1 1] Handle Swimming
  (`parent.ReceiveTick` DeltaSeconds)
  (if (not (`self.IsCharging`))
    (if (not (`self.IsPanicking`))
      (if (<= (`self.AttackCurrentCooldown`) 0.0)
        (`/Engine/EditorBlueprintResources/StandardMacros.IsValid` (`self.HauntedFish`)
          (:`Is Valid`
            (set `FloatingPawnMovement.MaxSpeed` (`self.SwimRandSpeed`) (`self.FloatingPawnMovement`))
            (`self.MoveTowardsLocation` (`self.K2_GetActorLocation` (`self.HauntedFish`)))
            (bind _inlightrange (`self.IsInLightRange`))
            (if _inlightrange
              (`self.SetupPanic`)
              (else
                (`self.FindNearbyFish`)))))
        (else
          (`self.HandleSwimAway`)))
      (else
        (`self.HandlePanic`)))
    (else
      (`self.HandleCharge`))))

(event `self.Attack`
  (params (Target :type "/Game/FishyJam/Core/BP_FishyFish Object Reference"))
  ;[1 1 1] Attack
  (`parent.Attack` Target))

(event `self.HandleWallHit`
  (set `self.IsPanicking` false))

(fn `CheckFishInRange`
  (`/Engine/EditorBlueprintResources/StandardMacros.IsValid` (`self.HauntedFish`)
    (:`Is Valid`
      (bind _inlightrange (`self.IsInLightRange`))
      (if (not _inlightrange)
        (bind _distance (`self.GetDistanceToPlayer`))
        (if (<= _distance (`self.ChargeRandDistance`))
          ;[1 1 1] CHARGE!
          (set `self.ChargeLocation` (`self.K2_GetActorLocation` (`self.HauntedFish`)))
          (set `self.IsCharging` true)
          (else
            ;[1 1 1] Check whether a FishyFriend is close by to eat
            (bind _fishyfriend (`self.CheckNearbyFishyFriend`))
            (`/Engine/EditorBlueprintResources/StandardMacros.IsValid` _fishyfriend
              (:`Is Valid`
                (set `self.ChargeLocation` (`self.K2_GetActorLocation` _fishyfriend))
                (set `self.IsCharging` true)))))))))

(fn `SetupPanic`
  (set `self.IsPanicking` true)
  (set `self.PanicDirection` (`KismetMathLibrary.Normal` (- (`self.K2_GetActorLocation`) (`self.K2_GetActorLocation` (`self.HauntedFish`)))))
  (set `self.PanicDistance` (`KismetMathLibrary.RandomFloatInRange` 500.0 2500.0))
  (set `self.PanicStartLocation` (`self.K2_GetActorLocation`)))

(fn `UserConstructionScript`)