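; Patrol enemy that moves toward randomly generated points and charges a BP_FishyFish that enters its interaction radius.
; The overlap stores the fish's position, then after a delay boosts speed and opens a Gate that lets Tick drive the charge.
; On arrival the Gate closes, and after a pause patrol speed returns.
; Advancing to the next patrol point is unwired, and hits only print a damage message.
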(event `self.ReceiveBeginPlay`
  (set `self.MaxSpeed` (`MovementComponent.GetMaxSpeed` (`self.FloatingPawnMovement`)))
  (`self.GeneratePatrolPoints`))

(event `self.ReceiveTick`
  (params (DeltaSeconds :type "Float (single-precision)"))
  ;[1 1 1] Handle Patrol Walk
  (`parent.ReceiveTick` DeltaSeconds)
  (if (not (`self.bIsCharging`))
    (bind _breached (`self.MoveTowardsLocation` (`|GetArrayItem` (`self.PatrolLocation`) (`self.CurrentPatrolLocation`))))
    (else
      (`/Engine/EditorBlueprintResources/StandardMacros.Gate` true :!label _label
        (:`Exit`
          (bind _breached_2 (`self.MoveTowardsLocation` (`self.ChargeLocation`)))
          (if _breached_2
            (`|ExecutionSequence`
              (:`then_0`
                (goto _label :!via `Close`))
              (:`then_1`
                (`KismetSystemLibrary.Delay` 1.0)
                (set `FloatingPawnMovement.MaxSpeed` (`self.MaxSpeed`) (`self.FloatingPawnMovement`))
                (set `self.bIsCharging` false)))))))))

(event `self.InteractionRadius.OnComponentBeginOverlap`
  (params (OverlappedComponent :type "PrimitiveComponent Object Reference") (OtherActor :type "Actor Object Reference") (OtherComp :type "PrimitiveComponent Object Reference") (OtherBodyIndex :type Integer) (bFromSweep :type Boolean) (SweepResult :type "HitResult Structure (by ref)"))
  (bind _asbp_fishy_fish (cast `/Game/FishyJam/Core/BP_FishyFish` OtherActor))
  (if (not (`self.bIsCharging`))
    (set `self.ChargeLocation` (`self.K2_GetActorLocation` _asbp_fishy_fish))
    (set `self.bIsCharging` true)
    (`KismetSystemLibrary.Delay` 1.0)
    (set `FloatingPawnMovement.MaxSpeed` (* 20.0 (`self.MaxSpeed`)) (`self.FloatingPawnMovement`))
    (goto _label :!via `Open`)))

(event `self.CollisionComponent_0.OnComponentHit`
  (params (HitComponent :type "PrimitiveComponent Object Reference") (OtherActor :type "Actor Object Reference") (OtherComp :type "PrimitiveComponent Object Reference") (NormalImpulse :type "Vector Structure") (Hit :type "HitResult Structure (by ref)"))
  (bind _asbp_fishy_fish (cast `/Game/FishyJam/Core/BP_FishyFish` OtherActor))
  (`KismetSystemLibrary.PrintString` (`KismetStringLibrary.Concat_StrStr` "Enemy: Deal damage to " (`KismetSystemLibrary.GetDisplayName` _asbp_fishy_fish))))

(fn `GeneratePatrolPoints`
  (if true
    (for _ (range (+ (`self.NumGenPatrolLocations`) 1))
      (`KismetArrayLibrary.Array_Add` (`self.PatrolLocation`) (`KismetMathLibrary.MakeVector` (`KismetMathLibrary.RandomFloatInRange` (`self.PatrolMinX`) (`self.PatrolMaxX`)) (`KismetMathLibrary.RandomFloatInRange` (`self.PatrolMinY`) (`self.PatrolMaxY`)) 100.0)))))

(fn `UserConstructionScript`)