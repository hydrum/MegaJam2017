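; Enemy fish pawn for FishyJam that hunts the player's fish and nearby not-yet-full FishyFriends, draining their energy on contact.
; BeginPlay randomizes speeds and charge range, while Tick smooths mesh rotation toward velocity and counts down attack cooldown.
; Helpers provide focus-charge-rest attacks, swimming away, panic and target search that avoids charging inside the player's energy-based light radius.
; This graph never calls those behavior helpers, and its wall-hit handler is empty.
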(event `self.ReceiveBeginPlay`
  ;[1 1 1] Set defaults
  (bind _output_get (set `self.SwimRandSpeed` (`KismetMathLibrary.RandomFloatInRange` 150.0 250.0)))
  (set `FloatingPawnMovement.MaxSpeed` _output_get (`self.FloatingPawnMovement`))
  (set `self.ChargeRandDistance` (`KismetMathLibrary.RandomFloatInRange` 300.0 400.0))
  (`self.RetrieveHauntedFish`)
  (set `self.ChargeRandSpeed` (* 10.0 (`self.SwimRandSpeed`)))
  (set `self.SwimAwayRandSpeed` (* 6.0 (`self.SwimRandSpeed`)))
  (set `self.PanicRandSpeed` (* 6.0 (`self.SwimRandSpeed`))))

(event `self.ReceiveTick`
  (params (DeltaSeconds :type "Float (single-precision)"))
  ;[1 1 1] Tick
  (`self.LerpRotation`)
  (set `self.AttackCurrentCooldown` (- (`self.AttackCurrentCooldown`) DeltaSeconds)))

(event `self.CollisionComponent.OnComponentHit`
  (params (HitComponent :type "PrimitiveComponent Object Reference") (OtherActor :type "Actor Object Reference") (OtherComp :type "PrimitiveComponent Object Reference") (NormalImpulse :type "Vector Structure") (Hit :type "HitResult Structure (by ref)"))
  (bind _asbp_fishy_fish (cast `/Game/FishyJam/Core/BP_FishyFish` OtherActor)
    (:`then`
      (if (<= (`self.AttackCurrentCooldown`) 0.0)
        (`self.Attack` _asbp_fishy_fish)
        (set `self.AttackCurrentCooldown` (`self.AttackCooldown`))))
    (:`CastFailed`
      (cast `ModelComponent` OtherComp)
      (`self.HandleWallHit`))))

(fn `Attack`
  (params (Target :type "/Game/FishyJam/Core/BP_FishyFish Object Reference"))
  (set `self.AttackedFish` Target)
  (bind _dealdamage_ (`self.CanDealDamage`))
  (if _dealdamage_
    (set `/Game/FishyJam/Core/BP_FishyFish.CurrentEnergy` (- (`/Game/FishyJam/Core/BP_FishyFish.CurrentEnergy` Target) (`self.AttackEnergyDamage`)) Target)
    (`/Game/FishyJam/Core/BP_FishyFish.DamageTaken` Target self (`self.AttackEnergyDamage`))))

(fn `CanDealDamage`
  (returns (`DealDamage?` :type Boolean))
  (bind _asbp_fishy_game_mode (cast `/Game/FishyJam/Core/GameModes/BP_FishyGameMode` (`GameplayStatics.GetGameMode`))
    (:`then`
      (if (`/Game/FishyJam/Core/GameModes/BP_FishyGameMode.bGameOver` _asbp_fishy_game_mode)
        _
        (else
          (return true))))
    (:`CastFailed`
      _))
  (return false))

(fn `CheckNearbyFishyFriend`
  (returns (FishyFriend :type "/Game/FishyJam/Core/Interactables/BP_FishyFriend Object Reference"))
  (bind _outactors (`GameplayStatics.GetAllActorsOfClass` "/Game/FishyJam/Core/Interactables/BP_FishyFriend.BP_FishyFriend_C"))
  (for _array_element _outactors
    (if (< (`/Game/FishyJam/Core/BP_FishyFish.CurrentEnergy` _array_element) (`/Game/FishyJam/Core/BP_FishyFish.MaxEnergy` _array_element))
      (if (>= (`self.ChargeRandDistance`) (`KismetMathLibrary.VSize` (- (`self.K2_GetActorLocation` _array_element) (`self.K2_GetActorLocation`))))
        (return _array_element))))
  (return null) ; return null
)

(fn `FindNearbyFish`
  (`/Engine/EditorBlueprintResources/StandardMacros.IsValid` (`self.HauntedFish`)
    (:`Is Valid`
      (bind _inlightrange (`self.IsInLightRange`))
      (if (not _inlightrange)
        (bind _distance (`self.GetDistanceToPlayer`))
        (if (<= _distance (`self.ChargeRandDistance`))
          ;[1 1 1] CHARGE!
          (set `self.ChargeLocation` (`self.K2_GetActorLocation` (`self.HauntedFish`)))
          (set `self.IsCharging` true)
          (else
            ;[1 1 1] Check whether a FishyFriend is close by to eat
            (bind _fishyfriend (`self.CheckNearbyFishyFriend`))
            (`/Engine/EditorBlueprintResources/StandardMacros.IsValid` _fishyfriend
              (:`Is Valid`
                (set `self.ChargeLocation` (`self.K2_GetActorLocation` _fishyfriend))
                (set `self.IsCharging` true)))))))))

(fn `GetDistanceToPlayer`
  (returns (Distance :type "Float (double-precision)"))
  (bind _hauntedfish (`self.HauntedFish`))
  (`/Engine/EditorBlueprintResources/StandardMacros.IsValid` _hauntedfish
    (:`Is Valid`
      (return (`KismetMathLibrary.VSize` (- (`self.K2_GetActorLocation` _hauntedfish) (`self.K2_GetActorLocation`)))))
    (:`Is Not Valid`
      (return -1.0))))

(fn `HandleCharge`
  (bind _chargelocaltimerrest (`self.ChargeLocalTimerRest`))
  (bind _chargelocaltimerfocus (`self.ChargeLocalTimerFocus`))
  (set `FloatingPawnMovement.MaxSpeed` (`self.ChargeRandSpeed`) (`self.FloatingPawnMovement`))
  ;[1 1 1] Let the fish focus at target
  (if (> _chargelocaltimerfocus 0.5)
    (if (`self.ChargeActuallyIsCharging`)
      (bind _breached (`self.MoveTowardsLocation` (`self.ChargeLocation`)))
      (set `self.ChargeActuallyIsCharging` (not _breached))
      (else
        ;[1 1 1] Rest
        (if (> _chargelocaltimerrest 0.2)
          (set `self.IsCharging` false)
          (`self.HandleChargeResetValues`)
          (else
            (set `self.ChargeLocalTimerRest` (+ _chargelocaltimerrest (`GameplayStatics.GetWorldDeltaSeconds`)))))))
    (else
      (set `self.ChargeLocalTimerFocus` (+ _chargelocaltimerfocus (`GameplayStatics.GetWorldDeltaSeconds`))))))

(fn `HandleChargeResetValues`
  (set `self.ChargeActuallyIsCharging` true)
  (set `self.ChargeLocalTimerRest` 0.0)
  (set `self.ChargeLocalTimerFocus` 0.0))

(fn `HandlePanic`
  (set `FloatingPawnMovement.MaxSpeed` (`self.PanicRandSpeed`) (`self.FloatingPawnMovement`))
  (bind _shouldstop (`self.HandlePanicEnough`))
  (if _shouldstop
    (set `self.IsPanicking` false)
    (else
      (`self.AddMovementInput` (`self.PanicDirection`)))))

(fn `HandlePanicEnough`
  (returns (ShouldStop :type Boolean))
  (return (>= (`KismetMathLibrary.VSize` (- (`self.K2_GetActorLocation`) (`self.PanicStartLocation`))) (`self.PanicDistance`))))

(fn `HandleSwimAway`
  (`/Engine/EditorBlueprintResources/StandardMacros.IsValid` (`self.AttackedFish`)
    (:`Is Valid`
      (`self.AddMovementInput` (`KismetMathLibrary.Normal` (- (`self.K2_GetActorLocation`) (`self.K2_GetActorLocation` (`self.AttackedFish`))))))))

(fn `HandleWallHit`)

(fn `IsInLightRange`
  (returns (InLightRange :type Boolean))
  (`/Engine/EditorBlueprintResources/StandardMacros.IsValid` (`self.HauntedFish`)
    (:`Is Valid`
      (bind _distance (`self.GetDistanceToPlayer`))
      (return (<= _distance (- (`/Game/FishyJam/Core/BP_FishyFish.CurrentEnergy` (`self.HauntedFish`)) 250.0))))
    (:`Is Not Valid`
      (return false))))

(fn `LerpRotation`
  (bind _floatingpawnmovement (`self.FloatingPawnMovement`))
  (bind (_returnvalue_x _returnvalue_y) (`KismetMathLibrary.BreakVector` (`KismetMathLibrary.Conv_RotatorToVector` (`self.K2_GetActorRotation`))))
  (bind (_velocity_x _velocity_y) (`KismetMathLibrary.BreakVector` (`MovementComponent.Velocity` (`self.FloatingPawnMovement`))))
  (if (!= (`MovementComponent.Velocity` _floatingpawnmovement) (0.0 0.0 0.0))
    (if (== (`KismetMathLibrary.CrossProduct2D` (`KismetMathLibrary.MakeVector2D` _velocity_x _velocity_y) (`KismetMathLibrary.MakeVector2D` _returnvalue_x _returnvalue_y)) 0.0)
      (`|ExecutionSequence`
        (:`then_0`
          (`SceneComponent.K2_AddRelativeRotation` (`self.Mesh`) (struct :`Yaw` 0.01) false false) ; if we look straight up or down, add a little more delta rot
        )
        (:`then_1`
          _)))
    (`SceneComponent.K2_SetRelativeRotation` (`self.Mesh`) (`KismetMathLibrary.Conv_VectorToRotator` (`KismetMathLibrary.Normal` (`KismetMathLibrary.VLerp` (`KismetMathLibrary.Conv_RotatorToVector` (`SceneComponent.RelativeRotation` (`self.Mesh`))) (`KismetMathLibrary.Normal` (`|Copy` (`MovementComponent.Velocity` _floatingpawnmovement))) 0.2))) false false) ; Need to lerp instead
  ))

(fn `MoveTowardsLocation`
  (params (Location :type "Vector Structure"))
  (returns (bReached :type Boolean))
  (bind _returnvalue (- Location (`self.K2_GetActorLocation`)))
  (`self.AddMovementInput` (`KismetMathLibrary.Normal` _returnvalue))
  (return (and (`KismetMathLibrary.NearlyEqual_FloatFloat` (.x _returnvalue) 0.0 50.0) (`KismetMathLibrary.NearlyEqual_FloatFloat` (.y _returnvalue) 0.0 50.0) (`KismetMathLibrary.NearlyEqual_FloatFloat` (.z _returnvalue) 0.0 50.0))))

(fn `RetrieveHauntedFish`
  (bind _asbp_fishy_pawn (cast `/Game/FishyJam/Core/Pawns/BP_FishyPawn` (`Controller.K2_GetPawn` (`GameplayStatics.GetPlayerController` 0)))
    (:`then`
      (set `self.HauntedFish` _asbp_fishy_pawn))
    (:`CastFailed`
      (`KismetSystemLibrary.K2_SetTimer` self "RetrieveHauntedFish" 0.1))))

(fn `UserConstructionScript`)