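; Piranha enemy that hunts the HauntedFish and flees once that fish moves faster than the game or menu mode's too-slow threshold.
; Each tick it chases at a randomized speed, or swims away during attack cooldown.
; Fleeing is permanent, at ten times speed, and destroys the actor once its screen projection leaves the viewport.
; Chomp audio plays randomly while chasing, fades on fleeing and stops at game over.
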(event `self.ReceiveBeginPlay`
  ;[1 1 1] BeginPlay
  (`parent.ReceiveBeginPlay`)
  (bind _output_get (set `self.SwimRandSpeed` (`KismetMathLibrary.RandomFloatInRange` 400.0 800.0)))
  (set `self.FleeingSpeed` (* _output_get 10.0)))

(event `self.ReceiveTick`
  (params (DeltaSeconds :type "Float (single-precision)"))
  (`parent.ReceiveTick` DeltaSeconds)
  (`/Engine/EditorBlueprintResources/StandardMacros.IsValid` (`self.HauntedFish`)
    (:`Is Valid`
      (`|ExecutionSequence`
        (:`then_0`
          ;[1 1 1] Mute chomp sound when gameover
          (bind _gameover_ (`self.IsGameOver`))
          (if _gameover_
            (`ActorComponent.Deactivate` (`self.AudioChomp`))))
        (:`then_1`
          (if (not (`self.bIsFleeing`))
            (if (<= (`self.AttackCurrentCooldown`) 0.0)
              (`self.SwimSpeedNormal`)
              (`self.MoveTowardsLocation` (`self.K2_GetActorLocation` (`self.HauntedFish`)))
              (`self.CheckFleeing`)
              ;[1 1 1] Play Chomp Sound
              (if (>= (`KismetMathLibrary.RandomFloatInRange` 0.0 1000.0) 998.0)
                (bind _gameover__2 (`self.IsGameOver`))
                (if (and (not (`AudioComponent.IsPlaying` (`self.AudioChomp`))) (not _gameover__2))
                  (`AudioComponent.Play` (`self.AudioChomp`) 0.0)))
              (else
                (`self.HandleSwimAway`)))
            (else
              (`self.HandleFleeing`)
              (`AudioComponent.FadeOut` (`self.AudioChomp`) 0.3 0.0)
              (`self.DestroyWhenOffscreen`))))))))

(fn `CheckFleeing`
  (`/Engine/EditorBlueprintResources/StandardMacros.IsValid` (`self.HauntedFish`)
    (:`Is Valid`
      (bind _asbp_fishy_game_mode (cast `/Game/FishyJam/Core/GameModes/BP_FishyGameMode` (`GameplayStatics.GetGameMode`))
        (:`then`
          (if (> (`KismetMathLibrary.VSize` (`MovementComponent.Velocity` (`/Game/FishyJam/Core/BP_FishyFish.FloatingPawnMovement` (`self.HauntedFish`)))) (`/Game/FishyJam/Core/GameModes/BP_FishyGameMode.TooSlowThreshold` _asbp_fishy_game_mode))
            (set `self.bIsFleeing` true :!label _label)))
        (:`CastFailed`
          (bind _asbp_fishy_menu_mode (cast `/Game/FishyJam/Core/GameModes/BP_FishyMenuMode` (`GameplayStatics.GetGameMode`)))
          (if (> (`KismetMathLibrary.VSize` (`MovementComponent.Velocity` (`/Game/FishyJam/Core/BP_FishyFish.FloatingPawnMovement` (`self.HauntedFish`)))) (`/Game/FishyJam/Core/GameModes/BP_FishyMenuMode.TooSlowThreshold` _asbp_fishy_menu_mode))
            (goto _label)))))))

(fn `DestroyWhenOffscreen`
  (bind (_returnvalue_x _returnvalue_y) (`KismetMathLibrary.BreakVector2D` (`WidgetLayoutLibrary.GetViewportSize`)))
  (bind _screenlocation (`PlayerController.ProjectWorldLocationToScreen` (`GameplayStatics.GetPlayerController` 0) (`self.K2_GetActorLocation`) false))
  (if (and (`self.bIsFleeing`) (not (and (> (`KismetMathLibrary.BreakVector2D` _screenlocation) 0.0) (> (`.Y` (`KismetMathLibrary.BreakVector2D` _screenlocation)) 0.0) (< (`KismetMathLibrary.BreakVector2D` _screenlocation) _returnvalue_x) (< (`.Y` (`KismetMathLibrary.BreakVector2D` _screenlocation)) _returnvalue_y))))
    (`self.K2_DestroyActor`)))

(fn `HandleFleeing`
  (set `FloatingPawnMovement.MaxSpeed` (`self.FleeingSpeed`) (`self.FloatingPawnMovement`))
  (`self.AddMovementInput` (`KismetMathLibrary.Normal` (- (`self.K2_GetActorLocation`) (`self.K2_GetActorLocation` (`self.HauntedFish`))))))

(fn `SwimSpeedNormal`
  (set `FloatingPawnMovement.MaxSpeed` (`self.SwimRandSpeed`) (`self.FloatingPawnMovement`)))

(fn `UserConstructionScript`)